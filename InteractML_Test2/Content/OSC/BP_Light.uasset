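; BP_Light is a light Blueprint whose point light brightness is driven by incoming OSC messages.
; The OSCMessage event stores the message and compares its full address path to the OSCAddress variable.
; On a match, UpdateLight reads the first float, clamps and remaps it from a unit range to a large intensity range, and sets the PointLight intensity.
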(event `/Game/OSC/BPI_OSCInterface.OSCMessage`
  (params (MessageContents :type "OSCMessage Structure"))
  (bind _output_get (set `self.Message Contents` MessageContents))
  (bind _returnvalue (`OSCManager.GetOSCMessageAddress` _output_get))
  (bind _returnvalue_2 (`OSCManager.GetOSCAddressFullPath` _returnvalue))
  (if (`KismetStringLibrary.EqualEqual_StrStr` _returnvalue_2 (`self.OSCAddress`))
    (`self.UpdateLight`)))

(event `UpdateLight`
  (bind _value (`OSCManager.GetFloat` (`self.Message Contents`)))
  (`LightComponent.SetIntensity` (`self.PointLight`) (`KismetMathLibrary.MapRangeClamped` _value 0.0 1.0 0.0 100000.0)))

(fn `UserConstructionScript`)