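; BP_OSCReciever receives Open Sound Control messages over the network and relays them to actors in the level.
; On BeginPlay it starts a listening OSC server on a hardcoded IP and port, then caches all actors implementing BPI_OSCInterface.
; Each received message is forwarded unparsed to those cached actors through the interface, leaving interpretation to them.
; Debug nodes for printing the address and first float are disconnected.
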(event `self.ReceiveBeginPlay`
  (bind _returnvalue (`OSCManager.CreateOSCServer` "100.126.56.124" 1337 false true "" null))
  (bind _output_get (set `self.OSCServer` _returnvalue))
  (add `OSCServer.OnOscMessageReceived` _output_get (`|CreateDelegate` :!event `OSCMessageReceived`))
  (bind _outactors (`GameplayStatics.GetAllActorsWithInterface` "/Game/OSC/BPI_OSCInterface.BPI_OSCInterface_C"))
  (set `self.OSCControlActors` _outactors))

(event `OSCMessageReceived`
  (params (Message :type "OSCMessage Structure (by ref)") (IPAddress :type String) (Port :type Integer))
  (message `/Game/OSC/BPI_OSCInterface.OSCMessage` (`self.OSCControlActors`) Message))

(fn `UserConstructionScript`)